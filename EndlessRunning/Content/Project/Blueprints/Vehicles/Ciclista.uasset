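; Ciclista is a cyclist actor that moves along the world Y axis and removes itself once the player has left it behind.
; Tick offsets it by Speed each frame, without delta-time scaling.
; A Delay inside Tick throttles the cleanup check to about every two seconds.
; That check destroys the actor when the Main_Character's Corpo component is at least 1000 units ahead in Y.
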(event `self.ReceiveTick`
  (params (DeltaSeconds :type "Float (single-precision)"))
  (bind (_returnvalue_x _returnvalue_y) (`KismetMathLibrary.BreakVector` (`self.K2_GetActorLocation`)))
  (`self.K2_AddActorWorldOffset` (`KismetMathLibrary.MakeVector` 0.0 (`self.Speed`)))
  (`KismetSystemLibrary.Delay` 2.0)
  (bind _asmain_character (cast `/Game/Project/Blueprints/Main_Character/Main_Character` (`GameplayStatics.GetPlayerCharacter` 0)))
  (bind (_returnvalue_x_2 _returnvalue_y_2) (`KismetMathLibrary.BreakVector` (`SceneComponent.K2_GetComponentLocation` (`/Game/Project/Blueprints/Main_Character/Main_Character.Corpo` _asmain_character))))
  (if (>= _returnvalue_y_2 (+ _returnvalue_y 1000.0))
    (`self.K2_DestroyActor`)))

(fn `UserConstructionScript`)