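; Vehicle actor that drives along world Y and destroys itself once the player character is 1500 units ahead of it.
; Construction picks a random row from the Veiculos data table, sets its mesh and applies random colors through dynamic material instances.
; Tick offsets it by Speed per frame, unscaled by delta time, and a Delay throttles the cleanup check to roughly every two seconds.
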(event `self.ReceiveTick`
  (params (DeltaSeconds :type "Float (single-precision)"))
  (bind (_returnvalue_x _returnvalue_y) (`KismetMathLibrary.BreakVector` (`self.K2_GetActorLocation`)))
  (`self.K2_AddActorWorldOffset` (`KismetMathLibrary.MakeVector` 0.0 (`self.Speed`)))
  (`KismetSystemLibrary.Delay` 2.0)
  (bind _asmain_character (cast `/Game/Project/Blueprints/Main_Character/Main_Character` (`GameplayStatics.GetPlayerCharacter` 0)))
  (bind (_returnvalue_x_2 _returnvalue_y_2) (`KismetMathLibrary.BreakVector` (`SceneComponent.K2_GetComponentLocation` (`/Game/Project/Blueprints/Main_Character/Main_Character.Corpo` _asmain_character))))
  (if (>= _returnvalue_y_2 (+ _returnvalue_y 1500.0))
    (`self.K2_DestroyActor`)))

(fn `UserConstructionScript`
  (bind _outrownames (`DataTableFunctionLibrary.GetDataTableRowNames` "/Game/Project/Dados/Veiculos/Veiculos.Veiculos"))
  (bind _returnvalue (`|GetDataTableRow` "/Game/Project/Dados/Veiculos/Veiculos.Veiculos" (`|GetArrayItem` _outrownames (`KismetMathLibrary.RandomIntegerInRange` 0 (- (`KismetArrayLibrary.Array_Length` _outrownames) 1))))
    (:`then`
      (bind (_mesh _cores) (break `/Game/Project/Dados/Veiculos/Structs/Veiculo` _returnvalue))
      (`StaticMeshComponent.SetStaticMesh` (`self.StaticMesh`) _mesh)
      (for _array_element _cores
        (bind (_nome _index _cores_2 _nomedomaterial) (break `/Game/Project/Dados/Veiculos/Structs/Veiculo_Cor` _array_element))
        (bind _returnvalue_2 (`PrimitiveComponent.CreateDynamicMaterialInstance` (`self.StaticMesh`) _index null "None"))
        (`MaterialInstanceDynamic.SetVectorParameterValue` _returnvalue_2 _nomedomaterial (`|GetArrayItem` _cores_2 (`KismetMathLibrary.RandomInteger` (- (`KismetArrayLibrary.Array_Length` _cores_2) 1))))))))