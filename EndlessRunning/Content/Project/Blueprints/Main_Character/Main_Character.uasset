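; Player character for a touch-controlled endless runner that hops forward along a column grid, dodging obstacles and collecting coins.
; Swipes set left/right flags; StartLoop picks the next cell, and timelines animate each hop, looping through BreakLoop.
; At edge columns a swipe can start a lane swap that turns and moves the character sideways.
; Death enables physics and saves coins; BreakLoop tracks score, saves highscores, updates the leaderboard and reloads the level.
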(event `self.ReceiveBeginPlay`
  ;[1 1 1] Initial Variables
  (`self.K2_AddActorWorldOffset` (0.0 0.0 -100.0) true) ; linha 800 coluna 1
  (`self.InitVariables`))

(event `InputAction|Finger1`
  (params (Key :type "Key Structure"))
  (bind (_locationx _locationy) (`PlayerController.GetInputTouchState` (`GameplayStatics.GetPlayerController` 0) "Touch1"))
  (bind (_returnvalue_roll _returnvalue_pitch _returnvalue_yaw) (`KismetMathLibrary.BreakRotator` (`SceneComponent.K2_GetComponentRotation` (`self.Corpo`))))
  (bind _returnvalue (`KismetMathLibrary.MakeVector2D` _locationx _locationy))
  ;[1 1 1] Input Touch
  (:`Pressed`
    (set `self.isTouched` true)
    (set `self.TouchLocationS` _locationx)
    (set `self.TouchStart` _returnvalue)
    (if (<= _locationy (`self.Yresolution`))
      ;[1 1 1] Start Playing
      (if (not (or (`self.Playing`) (`self.Skin`)))
        (set `self.Playing` true)
        (`WidgetLayoutLibrary.RemoveAllWidgets`)
        (bind _returnvalue_2 (`|CreateWidget` "/Game/Project/HUD/Menu/Gameplay.Gameplay_C"))
        (`UserWidget.AddToViewport` _returnvalue_2 0)
        ;[1 1 1] Movimentação do personagem
        (bind (_direction _lerpcamera) (`Timeline|MoveCam` :!via `PlayFromStart`)
          (:`Update`
            (`self.MoveCamera` _lerpcamera))
          (:`Finished`
            (`self.StartLoop` :!label _label)
            (`self.BreakLoop` :!label _label_2
              (:`then`
                (if (not (`KismetMathLibrary.BooleanNOR` (and (== (`self.Coluna`) 10) (`self.SwapLeft`) (`self.Swaping`)) (and (== (`self.Coluna`) 7) (not (`self.SwapLeft`)) (`self.Swaping`))))
                  ;[1 1 1] Return To Lane
                  (`KismetSystemLibrary.Delay` 0.3)
                  (if (and (`self.MoveLeft`) (== (`self.Coluna`) 10))
                    (set `self.ProxColuna` (+ (`self.Coluna`) 1))
                    (set `self.Swaping` false :!label _label_3)
                    (set `self.SwapLeft` false)
                    (set `self.MoveLeft` false)
                    (set `self.MoveRight` false)
                    (set `self.ProxLinha` (`self.Linha`))
                    (set `self.RotationBack` true)
                    (set `self.SwapAfterRotation` _returnvalue_yaw)
                    (elif (and (`self.MoveRight`) (== (`self.Coluna`) 7))
                      (set `self.ProxColuna` (- (`self.Coluna`) 1))
                      (goto _label_3)
                      (elif (and (`self.MoveRight`) (== (`self.Coluna`) 10))
                        (set `self.SwapLeft` false)
                        (set `self.ProxColuna` (- (`self.Coluna`) 1))
                        (set `self.SwapRotationDirection` 1.0)
                        (set `self.FlipRotation` -90.0)
                        (set `self.RotationSingle` true)
                        (elif (and (`self.MoveLeft`) (== (`self.Coluna`) 7))
                          (set `self.SwapLeft` true)
                          (set `self.ProxColuna` (+ (`self.Coluna`) 1))
                          (set `self.SwapRotationDirection` -1.0)
                          (set `self.FlipRotation` 90.0)
                          (set `self.RotationSingle` true)
                          (else
                            (if (`self.Swaping`) :!label _label_4
                              (`self.StartLoopWSwap`)
                              (goto _label_2)
                              (else
                                (goto _label)))))))))
                (if (`self.Swaping`)
                  (bind (_direction_2 _jumping _running) (`Timeline|MovementS` :!via `PlayFromStart`)
                    (:`Update`
                      (`self.SwapCharacter` _jumping _running
                        (:`then_1`
                          (`self.Camera_Position`))))
                    (:`Finished`
                      (bind (_direction_3 _scale) (`Timeline|Animacao` :!via `PlayFromStart` :!label _label_5)
                        (:`Update`
                          (`SceneComponent.SetWorldScale3D` (`self.Corpo`) (`KismetMathLibrary.MakeVector` 1.0 1.0 _scale)))
                        (:`Finished`
                          (goto _label_4)))))
                  (else
                    (bind (_direction_4 _jumping_2 _running_2) (`Timeline|Movement` :!via `PlayFromStart`)
                      (:`Update`
                        (`self.MoveCharacter` _jumping_2 _running_2
                          (:`then_1`
                            (`self.Camera_Position`))))
                      (:`Finished`
                        (goto _label_5 :!via `PlayFromStart`))))))
              (:`TimelineOut`
                (`Timeline|Tick` :!via `PlayFromStart`
                  (:`Update`
                    (goto _label_2 :!via `TimelineIn`))))))))))
  (:`Released`
    (set `self.isTouched` false)
    (goto _label_6 :!via `Reset`)))

(event `self.ReceiveTick`
  (params (DeltaSeconds :type "Float (single-precision)"))
  (bind (_locationx _locationy) (`PlayerController.GetInputTouchState` (`GameplayStatics.GetPlayerController` 0) "Touch1"))
  (bind _locationx_2 (`PlayerController.GetInputTouchState` (`GameplayStatics.GetPlayerController` 0) "Touch1"))
  (bind _returnvalue (`KismetMathLibrary.MakeVector2D` _locationx _locationy))
  ;[1 1 1] Input Touch
  (if (`self.isTouched`)
    (if (`self.Skin`)
      (`self.K2_AddActorLocalRotation` (`self.ActorSkin`) (`KismetMathLibrary.MakeRotator` 0.0 0.0 (- (`self.TouchLocationS`) _locationx_2)) false false)
      (set `self.TouchLocationS` _locationx_2)
      (elif (>= (`KismetMathLibrary.VSize2D` (- (`self.TouchStart`) _returnvalue)) 25.0)
        (`/Engine/EditorBlueprintResources/StandardMacros.DoOnce` false :!label _label_6
          (:`Completed`
            (bind _output_get (set `self.TouchEnd` _returnvalue))
            (bind (_x _y) (`KismetMathLibrary.BreakVector2D` (- (`self.TouchStart`) _output_get)))
            (if (>= (`KismetMathLibrary.Abs` _x) (`KismetMathLibrary.Abs` _y))
              (if (> _x 0.0)
                ;[1 1 1] Comando mover para os lados
                (`/Engine/EditorBlueprintResources/StandardMacros.Gate` false :!label _label_7 ; Left
                  (:`Exit`
                    (`|ExecutionSequence`
                      (:`then_0`
                        (goto _label_7 :!via `Close`))
                      (:`then_1`
                        (set `self.MoveLeft` true)
                        (set `self.MoveRight` false)
                        (`KismetSystemLibrary.Delay` 0.2)
                        (goto _label_7 :!via `Open`)))))
                (else
                  (`/Engine/EditorBlueprintResources/StandardMacros.Gate` false :!label _label_8 ; Right
                    (:`Exit`
                      (`|ExecutionSequence`
                        (:`then_0`
                          (goto _label_8 :!via `Close`))
                        (:`then_1`
                          (set `self.MoveRight` true)
                          (set `self.MoveLeft` false)
                          (`KismetSystemLibrary.Delay` 0.2)
                          (goto _label_8 :!via `Open`))))))))))))))

(event `self.Box.OnComponentBeginOverlap`
  (params (OverlappedComponent :type "PrimitiveComponent Object Reference") (OtherActor :type "Actor Object Reference") (OtherComp :type "PrimitiveComponent Object Reference") (OtherBodyIndex :type Integer) (bFromSweep :type Boolean) (SweepResult :type "HitResult Structure (by ref)"))
  (bind _returnvalue (`GameplayStatics.GetObjectClass` OtherActor))
  ;[1 1 1] Overlap
  (if (or (== _returnvalue "/Game/Project/Blueprints/NPCs/NPC_Default2.NPC_Default2_C") (== _returnvalue "/Game/Project/Blueprints/Vehicles/Veiculo.Veiculo_C") (== _returnvalue "/Game/Project/Blueprints/Vehicles/Ciclista.Ciclista_C") (== _returnvalue "/Game/Project/Blueprints/Level/Obstacles/ObstaclesCalcada.ObstaclesCalcada_C") (== _returnvalue "/Game/Project/Blueprints/Level/Obstacles/ObstacleNPC.ObstacleNPC_C"))
    (`self.GameOver` _returnvalue)
    (elif (== _returnvalue "/Game/Project/Blueprints/Colectables/Coin.Coin_C")
      (set `self.Coins` (+ (`self.Coins`) 1))
      (set `self.Pontuacao` (+ (`self.Pontuacao`) 2))
      (bind _asmain_game_mode (cast `/Game/Project/Main_GameMode` (`GameplayStatics.GetGameMode`)))
      (`/Game/Project/Blueprints/Assets/PoolClass/ObjectPool.DestroyFromPool` (`/Game/Project/Main_GameMode.PoolCoins` _asmain_game_mode) OtherActor)
      (`GameplayStatics.PlaySound2D` "/Game/Project/Assets/Audios/MenuPop.MenuPop" 1.0 1.0 0.0 null null))))

(event `Key|Z`
  (params (Key :type "Key Structure"))
  (:`Pressed`
    (`KismetSystemLibrary.ExecuteConsoleCommand` "stat game" null)))

(event `Key|X`
  (params (Key :type "Key Structure"))
  (:`Pressed`
    (`KismetSystemLibrary.ExecuteConsoleCommand` "stat gpu" null)))

(event `Key|C`
  (params (Key :type "Key Structure"))
  (:`Pressed`
    (`KismetSystemLibrary.ExecuteConsoleCommand` "stat unit" null)
    (`KismetSystemLibrary.ExecuteConsoleCommand` "stat fps" null)))

(event `Key|V`
  (params (Key :type "Key Structure"))
  (:`Pressed`
    (`/Engine/EditorBlueprintResources/StandardMacros.FlipFlop`
      (:`A`
        (`KismetSystemLibrary.ExecuteConsoleCommand` "stat startfile" null)
        (`KismetSystemLibrary.PrintString` "Started"))
      (:`B`
        (`KismetSystemLibrary.ExecuteConsoleCommand` "stat stopfile" null)
        (`KismetSystemLibrary.PrintString` "Stoped")))))

(fn `GameOver`
  (params (DeadBy :type "Actor Class Reference"))
  (if (not (`self.Dead`))
    (set `self.Dead` true)
    (`PrimitiveComponent.SetSimulatePhysics` (`self.Corpo`) true)
    (bind _returnvalue (`GameplayStatics.LoadGameFromSlot` "Save"))
    (bind _assave (cast `/Game/Project/Dados/Save` _returnvalue))
    (set `/Game/Project/Dados/Save.Coins` (`self.Coins`) _assave)
    (`GameplayStatics.SaveGameToSlot` _assave "Save")
    (if (== DeadBy "/Game/Project/Blueprints/Vehicles/Veiculo.Veiculo_C")
      (`GameplayStatics.PlaySoundAtLocation` "/Game/Project/Assets/Audios/Car_Beep.Car_Beep" (0.0 0.0 0.0) (struct) 1.0 1.0 0.0 null null null)
      (elif (== DeadBy "/Game/Project/Blueprints/Vehicles/Ciclista.Ciclista_C")
        (`GameplayStatics.PlaySoundAtLocation` "/Game/Project/Assets/Audios/BikeBell.BikeBell" (0.0 0.0 0.0) (struct) 1.0 1.0 0.0 null null null)))
    (`GameplayStatics.PlaySoundAtLocation` "/Game/Project/Assets/Audios/Fail.Fail" (0.0 0.0 0.0) (struct) 1.0 1.0 0.0 null null null)
    (bind _asmain_game_mode (cast `/Game/Project/Main_GameMode` (`GameplayStatics.GetGameMode`)))
    (bind _gamesound (`/Game/Project/Main_GameMode.GameSound` _asmain_game_mode))
    (if (`KismetSystemLibrary.IsValid` _gamesound)
      (`AudioComponent.Stop` _gamesound))))

(fn `UserConstructionScript`
  (bind _returnvalue (`GameplayStatics.LoadGameFromSlot` "Save"))
  (bind _assave (cast `/Game/Project/Dados/Save` _returnvalue))
  (bind (_corpo _pernas) (break `/Game/Project/Dados/SaveStruct` (`/Game/Project/Dados/Save.Equipado` _assave)))
  (`StaticMeshComponent.SetStaticMesh` (`self.Corpo`) _corpo)
  (`StaticMeshComponent.SetStaticMesh` (`self.Pernas`) _pernas))