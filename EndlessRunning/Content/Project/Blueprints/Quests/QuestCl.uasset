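; Quest controller that assigns a random quest on BeginPlay, tracking its ID, target quantity and current progress.
; CallQuest passes per-quest ranges to QuestsVar, which resets progress and rolls the target; the random pick only reaches quest IDs 2 and 3.
; CallType1 and CallType3 count progress, adding scaled or fixed points to Main_Character's Pontuacao on completion before rerolling.
; CallType2 rerolls immediately without reward.
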(event `self.ReceiveBeginPlay`
  (`self.CallQuest`))

(event `CallQuest`
  (switch `int` (`KismetMathLibrary.RandomIntegerInRange` 2 3)
    (:`0`
      (`self.QuestsVar` 10 30))
    (:`1`
      (`self.QuestsVar` 40 100 1))
    (:`2`
      (`self.QuestsVar` 500 600 2))
    (:`3`
      (`self.QuestsVar` 1 1 3))))

(event `CallType1`
  (bind _output_get (set `self.CurrentQtd` (+ (`self.CurrentQtd`) 1)))
  (if (>= _output_get (`self.QtdTotal`))
    (bind _asmain_character (cast `/Game/Project/Blueprints/Main_Character/Main_Character` (`GameplayStatics.GetPlayerCharacter` 0)))
    (set `/Game/Project/Blueprints/Main_Character/Main_Character.Pontuacao` (+ (`/Game/Project/Blueprints/Main_Character/Main_Character.Pontuacao` _asmain_character) (* (`self.QtdTotal`) 2)) _asmain_character)
    (`self.CallQuest`)))

(event `CallType2`
  (`self.CallQuest`))

(event `CallType3`
  (bind _output_get (set `self.CurrentQtd` (+ (`self.CurrentQtd`) 1)))
  (if (>= _output_get (`self.QtdTotal`))
    (bind _asmain_character (cast `/Game/Project/Blueprints/Main_Character/Main_Character` (`GameplayStatics.GetPlayerCharacter` 0)))
    (set `/Game/Project/Blueprints/Main_Character/Main_Character.Pontuacao` (+ (`/Game/Project/Blueprints/Main_Character/Main_Character.Pontuacao` _asmain_character) 100) _asmain_character)
    (`self.CallQuest`)))

(fn `QuestsVar`
  (params (RandomDown :type Integer) (RandomUp :type Integer) (QuestId :type Integer))
  (set `self.QtdTotal` (`KismetMathLibrary.RandomIntegerInRange` RandomDown RandomUp))
  (set `self.CurrentQtd` 0)
  (set `self.CurrentQuest` QuestId)
  (cast `/Game/Project/Blueprints/Main_Character/Main_Character` (`GameplayStatics.GetPlayerCharacter` 0)))