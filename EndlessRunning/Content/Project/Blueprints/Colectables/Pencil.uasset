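; Pencil collectable actor that spins in place and cleans itself up once the player has moved well past it along Y.
; Tick adds a fixed yaw step every frame, so spin speed depends on frame rate.
; A Delay in Tick throttles the check comparing the Main_Character's Corpo component position to the pencil's, which destroys the actor.
; No pickup or overlap logic is implemented here.
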(event `self.ReceiveTick`
  (params (DeltaSeconds :type "Float (single-precision)"))
  (bind (_returnvalue_x _returnvalue_y) (`KismetMathLibrary.BreakVector` (`self.K2_GetActorLocation`)))
  (bind (_returnvalue_roll _returnvalue_pitch _returnvalue_yaw) (`KismetMathLibrary.BreakRotator` (`self.K2_GetActorRotation`)))
  (`self.K2_SetActorRotation` (`KismetMathLibrary.MakeRotator` _returnvalue_roll _returnvalue_pitch (+ _returnvalue_yaw 5.0)))
  (`KismetSystemLibrary.Delay` 2.0)
  (bind _asmain_character (cast `/Game/Project/Blueprints/Main_Character/Main_Character` (`GameplayStatics.GetPlayerCharacter` 0)))
  (bind (_returnvalue_x_2 _returnvalue_y_2) (`KismetMathLibrary.BreakVector` (`SceneComponent.K2_GetComponentLocation` (`/Game/Project/Blueprints/Main_Character/Main_Character.Corpo` _asmain_character))))
  (if (>= _returnvalue_y_2 (+ _returnvalue_y 1500.0))
    (`self.K2_DestroyActor`)))

(fn `UserConstructionScript`)