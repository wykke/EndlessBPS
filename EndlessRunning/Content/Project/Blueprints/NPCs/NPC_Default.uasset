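; NPC that randomizes its look, hops endlessly along -Y one step at a time, and destroys itself once far behind Main_Character.
; Construction Script builds it from per-part data tables, setting meshes and randomly colored dynamic materials, sharing skin and shirt colors across parts.
; Head and body rows gate the optional hat and sleeve type; accessories are random extras.
; Looping timelines drive each swept hop, then a capsule Z-scale squash.
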(event `self.ReceiveBeginPlay`
  (bind (_returnvalue_x _returnvalue_y _returnvalue_z) (`KismetMathLibrary.BreakVector` (`self.K2_GetActorLocation`)))
  (bind (_returnvalue_x_2 _returnvalue_y_2) (`KismetMathLibrary.BreakVector` (`self.K2_GetActorLocation`)))
  (bind (_returnvalue_x_3 _returnvalue_y_3) (`KismetMathLibrary.BreakVector` (`self.K2_GetActorLocation`)))
  (set `self.ProxLinha` _returnvalue_y_3)
  (`KismetSystemLibrary.Delay` 0.1)
  (bind _output_get (set `self.Linha` (`self.ProxLinha`) :!label _label)) ; Inicio Do Loop
  (set `self.ProxLinha` (+ _output_get -100.0))
  (bind (_direction _jumping _running) (`Timeline|Timeline_0` :!via `PlayFromStart`)
    (:`Update`
      (`|ExecutionSequence`
        (:`then_0`
          (`self.K2_AddActorWorldOffset` (`KismetMathLibrary.MakeVector` 0.0 0.0 (* _jumping (`self.JumpHeight`))) true))
        (:`then_1`
          (`self.K2_SetActorLocation` (`KismetMathLibrary.MakeVector` _returnvalue_x (`KismetMathLibrary.Lerp` (`self.Linha`) (`self.ProxLinha`) _running) _returnvalue_z) true)
          (bind _outactors (`GameplayStatics.GetAllActorsOfClass` "/Game/Project/Blueprints/Main_Character/Main_Character.Main_Character_C"))
          (bind _asmain_character (cast `/Game/Project/Blueprints/Main_Character/Main_Character` (`|GetArrayItem` _outactors)))
          (bind (_returnvalue_x_4 _returnvalue_y_4) (`KismetMathLibrary.BreakVector` (`self.K2_GetActorLocation` _asmain_character)))
          (if (>= _returnvalue_y_4 (+ _returnvalue_y_2 2000.0))
            (`self.K2_DestroyActor`)))))
    (:`Finished`
      (bind (_direction_2 _scale) (`Timeline|Timeline_1` :!via `PlayFromStart`)
        (:`Update`
          (`SceneComponent.SetWorldScale3D` (`self.CapsuleComponent`) (`KismetMathLibrary.MakeVector` 1.0 1.0 _scale)))
        (:`Finished`
          (goto _label))))))

(fn `UserConstructionScript`
  (`self.RandomPele`
    (:`Out`
      (bind _chapeu (`self.RandomCabeca`)
        (:`Out`
          (if (and _chapeu (<= (`KismetMathLibrary.RandomIntegerInRange` 1 10) 3))
            (`self.RandomChapeu`
              (:`Out`
                _)))
          (bind _mangacomprida (`self.RandomCorpo`)
            (:`Out`
              (if _mangacomprida
                (`self.RandomBracoC`
                  (:`Out`
                    _))
                (else
                  (`self.RandomBraco`
                    (:`Out`
                      _))))
              (`self.RandomPernas`
                (:`Out`
                  (`self.RandomPes`
                    (:`Out`
                      (switch `int` (`KismetMathLibrary.RandomIntegerInRange` 0 2)
                        (:`1`
                          _)
                        (:`2`
                          (`self.RandomAcessório2`
                            (:`Out`
                              _))))
                      (`self.RandomAcessório1`))))))))))))