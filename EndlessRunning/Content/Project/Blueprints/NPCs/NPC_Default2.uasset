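; NPC that hops along -Y in 100-unit steps and randomizes its modular look at construction.
; Construction picks gender and skin tone, then fills body-part meshes and colors from gendered DataTables; torso dictates sleeve type and shirt color, head permits hats.
; Timelines drive each hop and foot squash, looping until a check every fourth hop finds it 1000+ units past the player.
; Accessory slot 1 always loads "OculosRedondo1", ignoring its random pick.
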(event `self.ReceiveBeginPlay`
  (bind (_returnvalue_x _returnvalue_y _returnvalue_z) (`KismetMathLibrary.BreakVector` (`self.K2_GetActorLocation`)))
  (bind (_returnvalue_x_2 _returnvalue_y_2) (`KismetMathLibrary.BreakVector` (`self.K2_GetActorLocation`)))
  (bind (_returnvalue_x_3 _returnvalue_y_3) (`KismetMathLibrary.BreakVector` (`self.K2_GetActorLocation`)))
  (set `self.ProxLinha` _returnvalue_y_3)
  (if (`self.Auto`)
    (`KismetSystemLibrary.Delay` (`KismetMathLibrary.RandomFloatInRange` 0.0 1.0)))
  (bind _output_get (set `self.Linha` (`self.ProxLinha`) :!label _label)) ; Inicio Do Loop
  (set `self.ProxLinha` (+ _output_get -100.0))
  (bind (_direction _jumping _running) (`Timeline|Timeline_1` :!via `PlayFromStart`)
    (:`Update`
      (`self.K2_AddActorWorldOffset` (`KismetMathLibrary.MakeVector` 0.0 0.0 _jumping) true)
      (`self.K2_SetActorLocation` (`KismetMathLibrary.MakeVector` _returnvalue_x (`KismetMathLibrary.Lerp` (`self.Linha`) (`self.ProxLinha`) _running) _returnvalue_z)))
    (:`Finished`
      (bind (_direction_2 _scale) (`Timeline|Timeline_0` :!via `PlayFromStart`)
        (:`Update`
          (`SceneComponent.SetWorldScale3D` (`self.pes`) (`KismetMathLibrary.MakeVector` 1.0 1.0 _scale)))
        (:`Finished`
          (`/Engine/EditorBlueprintResources/StandardMacros.FlipFlop`
            (:`A`
              (`/Engine/EditorBlueprintResources/StandardMacros.FlipFlop`
                (:`A`
                  (bind _asmain_character (cast `/Game/Project/Blueprints/Main_Character/Main_Character` (`GameplayStatics.GetPlayerCharacter` 0)))
                  (bind (_returnvalue_x_4 _returnvalue_y_4) (`KismetMathLibrary.BreakVector` (`SceneComponent.K2_GetComponentLocation` (`/Game/Project/Blueprints/Main_Character/Main_Character.Corpo` _asmain_character))))
                  (if (>= _returnvalue_y_4 (+ _returnvalue_y_2 1000.0))
                    (`self.K2_DestroyActor`)
                    (else
                      (goto _label))))
                (:`B`
                  (goto _label))))
            (:`B`
              (goto _label))))))))

(fn `UserConstructionScript`
  (set `self.Female` (== (`KismetMathLibrary.RandomIntegerInRange` 0 1) 0))
  (`self.RandomPele`
    (:`Out`
      (bind _chapeu (`self.RandomCabeca`)
        (:`Out`
          (if (and _chapeu (<= (`KismetMathLibrary.RandomIntegerInRange` 1 10) 3))
            (`self.RandomChapeu`
              (:`Out`
                _)))
          (bind _mangacomprida (`self.RandomCorpo`)
            (:`Out`
              (if _mangacomprida
                (`self.RandomBracoC`
                  (:`Out`
                    _))
                (else
                  (`self.RandomBraco`
                    (:`Out`
                      _))))
              (`self.RandomPernas`
                (:`Out`
                  (`self.RandomPes`
                    (:`Out`
                      (switch `int` (`KismetMathLibrary.RandomIntegerInRange` 0 2)
                        (:`1`
                          _)
                        (:`2`
                          (`self.RandomAcessorio2`
                            (:`Out`
                              _))))
                      (`self.RandomAcessorio1`))))))))))))